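; Trigger-driven door that rises when a BP_Character enters its EnterTrigger and lowers when one leaves.
; A timeline drives the door's relative Z from the height stored at BeginPlay up to MaxOpenHeight above it, reversing on exit.
; IsDoorOpen guards the opening but is cleared on every timeline update, so re-entry restarts from the start.
; Opening and Closing events are empty.
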(event OnComponentBeginOverlap(EnterTrigger)
  (params (OverlappedComponent :type Primitive%20Component%20Object%20Reference) (OtherActor :type Actor%20Object%20Reference) (OtherComp :type Primitive%20Component%20Object%20Reference) (OtherBodyIndex :type Integer) (bFromSweep :type Boolean) (SweepResult :type Hit%20Result%20Structure%20%28by%20ref%29))
  (bind _reltive_location_z (Variables|Default|GetReltive%20Location%20Z))
  (Utilities|Casting|CastToBP_Character OtherActor)
  (if (not (Variables|Default|GetbIsDoorOpen))
    (Variables|Default|SetbIsDoorOpen true)
    (bind _zoffset (Timeline|Timeline_0 PlayFromStart)
      (:Update
        (Transformation|SetRelativeLocation (Variables|Default|GetDoor) (Math|Vector|MakeVector 0.0 0.0 (Math|Float|MapRangeClamped _zoffset 0.0 1.0 _reltive_location_z (+ _reltive_location_z (Variables|Default|GetMaxOpenHeight)))) false false)
        (Variables|Default|SetbIsDoorOpen false)))))

(event OnComponentEndOverlap(EnterTrigger)
  (params (OverlappedComponent :type Primitive%20Component%20Object%20Reference) (OtherActor :type Actor%20Object%20Reference) (OtherComp :type Primitive%20Component%20Object%20Reference) (OtherBodyIndex :type Integer))
  (bind _reltive_location_z (Variables|Default|GetReltive%20Location%20Z))
  (Utilities|Casting|CastToBP_Character OtherActor)
  (bind _zoffset (Timeline|Timeline_0 Reverse)
    (:Update
      (Transformation|SetRelativeLocation (Variables|Default|GetDoor) (Math|Vector|MakeVector 0.0 0.0 (Math|Float|MapRangeClamped _zoffset 0.0 1.0 _reltive_location_z (+ _reltive_location_z (Variables|Default|GetMaxOpenHeight)))) false false)
      (Variables|Default|SetbIsDoorOpen false))))

(event Custom|Opening)

(event Custom|Closing)

(event EventBeginPlay
  (Variables|Default|SetReltive%20Location%20Z (.z (Variables|/Script/Engine.SceneComponent|GetRelativeLocation (Variables|Default|GetDoor)))))

(event Collision|EventActorBeginOverlap
  (params (OtherActor :type Actor%20Object%20Reference)))

(event EventTick
  (params (DeltaSeconds :type Float%20%28single-precision%29)))

(fn ConstructionScript)